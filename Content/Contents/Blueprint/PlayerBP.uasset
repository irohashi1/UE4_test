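; Player character Blueprint that flies forward automatically and is steered by device tilt, with keyboard and look axes also bound.
; Each Tilt event stores the gyro value, turns it into controller yaw and pitch, sets max fly speed, then adds forward input along the control rotation, pitch included.
; Axis bindings add yaw-only planar movement and camera look.
; An alternative tilt-threshold movement function exists but is never executed.
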(event `InputAxis|MoveFoward`
  (params (AxisValue :type "Float (single-precision)"))
  ;[1 1 1] Movement Character Keyboard
  (`self.AddMovementInput` (`KismetMathLibrary.GetForwardVector` (`KismetMathLibrary.MakeRotator` 0.0 0.0 (.yaw (`self.GetControlRotation`)))) AxisValue))

(event `InputVectorAxis|Tilt`
  (params (AxisValue :type "Vector Structure"))
  ;[1 1 1] Movement
  (set `self.Jyro Axis Value` AxisValue)
  (`|ExecutionSequence`
    (:`then_0`
      (`self.Camera Jyro`)
      (`self.Speed`))
    (:`then_1`
      (`self.Movement Character`))))

(event `InputAxis|MoveRight`
  (params (AxisValue :type "Float (single-precision)"))
  ;[1 1 1] Movement Character Keyboard
  (`self.AddMovementInput` (`KismetMathLibrary.GetRightVector` (`KismetMathLibrary.MakeRotator` 0.0 0.0 (.yaw (`self.GetControlRotation`)))) AxisValue))

(event `InputAxis|Turn`
  (params (AxisValue :type "Float (single-precision)"))
  ;[1 1 1] Movement Camera
  (`self.AddControllerYawInput` AxisValue))

(event `InputAxis|LookUp`
  (params (AxisValue :type "Float (single-precision)"))
  ;[1 1 1] Movement Camera
  (`self.AddControllerPitchInput` AxisValue))

(event `InputAxis|TurnRate`
  (params (AxisValue :type "Float (single-precision)"))
  ;[1 1 1] Movement Camera
  (`self.AddControllerYawInput` AxisValue))

(event `InputAxis|LookUpRate`
  (params (AxisValue :type "Float (single-precision)"))
  ;[1 1 1] Movement Camera
  (`self.AddControllerPitchInput` AxisValue))

(fn `Camera Jyro`
  (`|ExecutionSequence`
    (:`then_0`
      ;[1 1 1] Yaw
      (`self.AddControllerYawInput` (* (`KismetMathLibrary.DegreesToRadians` (* (`KismetMathLibrary.RadiansToDegrees` (.z (`self.Jyro Axis Value`))) -1.0)) 2.5)))
    (:`then_1`
      ;[1 1 1] Pitch
      (`self.AddControllerPitchInput` (* (`KismetMathLibrary.DegreesToRadians` (+ (`KismetMathLibrary.RadiansToDegrees` (.x (`self.Jyro Axis Value`))) 0.0)) 2.5)))))

(fn `Movement Character`
  (`self.AddMovementInput` (`KismetMathLibrary.GetForwardVector` (`KismetMathLibrary.MakeRotator` 0.0 (.pitch (`self.GetControlRotation`)) (.yaw (`self.GetControlRotation`)))) 1.0))

(fn `Movement Jyro`
  (bind _returnvalue (`KismetMathLibrary.RadiansToDegrees` (.x (`self.Jyro Axis Value`))))
  (if (> _returnvalue -30.0)
    (`self.AddMovementInput` (`KismetMathLibrary.GetForwardVector` (`KismetMathLibrary.MakeRotator` 0.0 0.0 (.yaw (`self.GetControlRotation`)))) (/ (+ _returnvalue 30.0) 1.0))))

(fn `Speed`
  (set `CharacterMovementComponent.MaxFlySpeed` 500.0 (`self.CharacterMovement`)))

(fn `UserConstructionScript`)