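; Countdown time-limit Blueprint that creates and displays a TimeLimitWD widget on BeginPlay, passing it a self reference.
; Tick watches a one-shot TimeLimitStart flag and launches a looping millisecond-interval TimeCount timer.
; TimeCount chains CalcTime borrows from milliseconds through seconds to minutes and builds the DrawTime string.
; When minutes underflow, it sets IsEnd and zeroes the time, without clearing the timer.
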(event `self.ReceiveBeginPlay`
  (bind _returnvalue (`|CreateWidget` "/Game/Contents/Blueprint/Widget/TimeLimitWD.TimeLimitWD_C"))
  (set `self.TimeLimitWDRef` _returnvalue)
  (set `/Game/Contents/Blueprint/Widget/TimeLimitWD.TimeLimitRef` self _returnvalue)
  (`UserWidget.AddToViewport` _returnvalue 0))

(event `self.ReceiveTick`
  (params (DeltaSeconds :type "Float (single-precision)"))
  (if (`self.TimeLimitStart`)
    (set `self.TimeLimitStart` false)
    (set `self.IsTimeCount` true)
    (`KismetSystemLibrary.K2_SetTimer` null "TimeCount" 0.001 true)))

(fn `CalcTime`
  (params (Time :type Integer) (AddTime :type Integer) (Max :type Integer))
  (returns (Up :type Integer) (UpdateTime :type Integer))
  (bind _returnvalue (- Time AddTime))
  (if (< _returnvalue 0)
    (return 1 Max)
    (else
      (return 0 _returnvalue))))

(fn `TimeCount`
  ;[1 1 1] ミリ秒
  (bind (_up _updatetime) (`self.CalcTime` (`self.Time_msec`) (`self.AddTime`) 999))
  (set `self.Time_msec` _updatetime)
  ;[1 1 1] 秒
  (bind (_up_2 _updatetime_2) (`self.CalcTime` (`self.Time_sec`) _up 59))
  (set `self.Time_sec` _updatetime_2)
  ;[1 1 1] 分
  (bind (_up_3 _updatetime_3) (`self.CalcTime` (`self.Time_min`) _up_2 59))
  (set `self.Time_min` _updatetime_3)
  (if (< 0 _up_3)
    ;[1 1 1] 制限時間過ぎ
    (set `self.IsEnd` true)
    (set `self.Time_min` 0)
    (set `self.Time_sec` 0)
    (set `self.Time_msec` 0))
  (set `self.DrawTime` (`KismetStringLibrary.Concat_StrStr` (`KismetStringLibrary.Conv_IntToString` (`self.Time_min`)) ":" (`KismetStringLibrary.Conv_IntToString` (`self.Time_sec`)) ":" (`KismetStringLibrary.Conv_IntToString` (`self.Time_msec`)))))

(fn `UserConstructionScript`)