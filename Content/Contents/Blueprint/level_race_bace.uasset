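; Level script for a race stage that runs the race from countdown to return to the title level.
; BeginPlay registers the pause manager with the game instance, shows the race HUD and countdown widget, and locks player input.
; Tick drives a state machine: countdown end unlocks input, starts BGM and the time limit.
; When time expires, it shows the end widget, disables input, and after a delay loads level_title.
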(event `self.ReceiveBeginPlay`
  (bind _characterbpref (`self.CharacterBPRef`))
  ;[1 1 1] Pause
  (bind _asmy_game_instance (cast `/Game/Contents/Blueprint/MyGameInstance` (`GameplayStatics.GetGameInstance`)))
  (set `/Game/Contents/Blueprint/MyGameInstance.PauseManagerRef` (`self.PauseManagerRef`) _asmy_game_instance)
  ;[1 1 1] Create Race UMG
  (bind _returnvalue (`|CreateWidget` "/Game/Contents/Blueprint/Widget/Race_WD.Race_WD_C"))
  (`UserWidget.AddToViewport` _returnvalue 0)
  ;[1 1 1] Player Init
  (set `self.State` "NewEnumerator0")
  (set `/Game/Contents/Blueprint/CharacterBP.Check Point Flag` false _characterbpref)
  (set `/Game/Contents/Blueprint/CharacterBP.Input Flag` false _characterbpref)
  ;[1 1 1] Count Down Start
  (set `self.State` "NewEnumerator1")
  (bind _returnvalue_2 (`|CreateWidget` "/Game/Contents/Blueprint/Widget/CountDownWD.CountDownWD_C"))
  (set `self.CountDownHUD` _returnvalue_2)
  (`UserWidget.AddToViewport` _returnvalue_2 0))

(event `self.ReceiveTick`
  (params (DeltaSeconds :type "Float (single-precision)"))
  ;[1 1 1] Race Flow
  (switch `/Game/Contents/Blueprint/level_race_bace_EN` (`self.State`)
    (:`NewEnumerator1`
      ;[1 1 1] CountDown End
      (if (`/Game/Contents/Blueprint/Widget/CountDownWD.IsCountEnd` (`self.CountDownHUD`))
        (set `/Game/Contents/Blueprint/CharacterBP.Input Flag` true (`self.CharacterBPRef`))
        (set `self.State` "NewEnumerator2")
        (`GameplayStatics.PlaySound2D` (`self.Bgm`))
        (set `/Game/Contents/Blueprint/TimeLimitBP.TimeLimitStart` true (`self.TimeLimitBPRef`))))
    (:`NewEnumerator2`
      ;[1 1 1] Race
      (if (`/Game/Contents/Blueprint/TimeLimitBP.IsEnd` (`self.TimeLimitBPRef`))
        (set `self.State` "NewEnumerator3")
        (bind _returnvalue (`|CreateWidget` "/Game/Contents/Blueprint/Widget/RaceEnd_WD.RaceEnd_WD_C"))
        (`UserWidget.AddToViewport` _returnvalue 0)
        (set `/Game/Contents/Blueprint/CharacterBP.Input Flag` false (`self.CharacterBPRef`))))
    (:`NewEnumerator3`
      ;[1 1 1] Go To Result
      (`KismetSystemLibrary.Delay` 3.0)
      (bind _asmy_game_instance (cast `/Game/Contents/Blueprint/MyGameInstance` (`GameplayStatics.GetGameInstance`)))
      (`/Game/Contents/Blueprint/MyGameInstance.StateLevel` _asmy_game_instance "level_title"))))

(fn `UserConstructionScript`)