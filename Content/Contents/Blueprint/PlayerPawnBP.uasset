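; PlayerPawnBP is a player pawn with keyboard movement and camera control from both look axes and device tilt.
; Move inputs follow the control rotation's yaw only, while turn and look axes feed controller yaw and pitch directly.
; Tilt stores its value for JyroCamera, which adds scaled yaw from inverted Z and pitch from X; its radian-degree round trips cancel out.
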(event `InputVectorAxis|Tilt`
  (params (AxisValue :type "Vector Structure"))
  ;[1 1 1] Movement
  (set `self.Jyro Value` AxisValue)
  (`|ExecutionSequence`
    (:`then_0`
      (`self.Jyro Camera`))))

(event `InputAxis|Turn`
  (params (AxisValue :type "Float (single-precision)"))
  ;[1 1 1] Movement Camera
  (`self.AddControllerYawInput` AxisValue))

(event `InputAxis|LookUp`
  (params (AxisValue :type "Float (single-precision)"))
  ;[1 1 1] Movement Camera
  (`self.AddControllerPitchInput` AxisValue))

(event `InputAxis|TurnRate`
  (params (AxisValue :type "Float (single-precision)"))
  ;[1 1 1] Movement Camera
  (`self.AddControllerYawInput` AxisValue))

(event `InputAxis|LookUpRate`
  (params (AxisValue :type "Float (single-precision)"))
  ;[1 1 1] Movement Camera
  (`self.AddControllerPitchInput` AxisValue))

(event `InputAxis|MoveFoward`
  (params (AxisValue :type "Float (single-precision)"))
  ;[1 1 1] Movement Character Keyboard
  (`self.AddMovementInput` (`KismetMathLibrary.GetForwardVector` (`KismetMathLibrary.MakeRotator` 0.0 0.0 (.yaw (`self.GetControlRotation`)))) AxisValue))

(event `InputAxis|MoveRight`
  (params (AxisValue :type "Float (single-precision)"))
  ;[1 1 1] Movement Character Keyboard
  (`self.AddMovementInput` (`KismetMathLibrary.GetRightVector` (`KismetMathLibrary.MakeRotator` 0.0 0.0 (.yaw (`self.GetControlRotation`)))) AxisValue))

(fn `Jyro Camera`
  (`|ExecutionSequence`
    (:`then_0`
      ;[1 1 1] Yaw
      (`self.AddControllerYawInput` (* (`KismetMathLibrary.DegreesToRadians` (* (`KismetMathLibrary.RadiansToDegrees` (.z (`self.Jyro Value`))) -1.0)) 2.5)))
    (:`then_1`
      ;[1 1 1] Pitch
      (`self.AddControllerPitchInput` (* (`KismetMathLibrary.DegreesToRadians` (+ (`KismetMathLibrary.RadiansToDegrees` (.x (`self.Jyro Value`))) 0.0)) 2.5)))))

(fn `UserConstructionScript`)