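; PauseManager is an actor Blueprint that toggles the game's pause state and pause menu.
; On BeginPlay it creates a PauseMenuWD widget once and caches the reference.
; Pause_Event calls ChangePause, which flips IsPause, adds or removes the cached widget from the viewport, and sets the game paused to match.
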(event `self.ReceiveBeginPlay`
  (bind _returnvalue (`|CreateWidget` "/Game/Contents/Blueprint/PauseMenuWD.PauseMenuWD_C"))
  (set `self.PauseMenuWDRef` _returnvalue))

(event `self.ReceiveTick`
  (params (DeltaSeconds :type "Float (single-precision)"))
  (if true
    _))

(event `Pause_Event`
  (`self.ChangePause`))

(fn `ChangePause`
  (bind _pausemenuwdref (`self.PauseMenuWDRef`))
  (if (`self.IsPause`)
    (set `self.IsPause` false)
    (`Widget.RemoveFromParent` _pausemenuwdref)
    (`GameplayStatics.SetGamePaused` false)
    (else
      (set `self.IsPause` true)
      (`UserWidget.AddToViewport` _pausemenuwdref 0)
      (`GameplayStatics.SetGamePaused` true))))

(fn `UserConstructionScript`)