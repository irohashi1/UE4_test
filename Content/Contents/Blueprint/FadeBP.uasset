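; FadeBP is an actor Blueprint that handles screen fades and the jump to the loading level.
; On BeginPlay it registers itself with MyGameInstance, creates the FadeWD widget and triggers a fade-in.
; Fade events play the widget's In and Out animations, whose finished callbacks set completion flags; fade-in also removes the widget.
; Tick opens "level_load" once the game instance's JumpLevel flag is set and the fade-out has finished.
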(event `self.ReceiveBeginPlay`
  ;[1 1 1] State SetUp
  (bind _asmy_game_instance (cast `/Game/Contents/Blueprint/MyGameInstance` (`GameplayStatics.GetGameInstance`)))
  (set `/Game/Contents/Blueprint/MyGameInstance.FadeBP` self _asmy_game_instance)
  ;[1 1 1] WD Set Up
  (bind _returnvalue (`|CreateWidget` "/Game/Contents/Blueprint/Widget/FadeWD.FadeWD_C"))
  (set `self.WD_Fade` _returnvalue)
  (set `self.Anime_FadeIn` (`/Game/Contents/Blueprint/Widget/FadeWD.In` _returnvalue))
  (set `self.Anime_FadeOut` (`/Game/Contents/Blueprint/Widget/FadeWD.Out` _returnvalue))
  (`UserWidget.AddToViewport` (`self.WD_Fade`) 0)
  (`self.FadeIn_Event`))

(event `FadeIn_Event`
  ;[1 1 1] Fade In
  (`UserWidget.PlayAnimation` (`self.WD_Fade`) (`self.Anime_FadeIn`) 0.0 1 "Forward" 1.0)
  (add `WidgetAnimation.OnAnimationFinished` (`self.Anime_FadeIn`) (delegate `Event_AnimeFIn_FadeIn`)))

(event `FadeOut_Event`
  ;[1 1 1] Fade Out
  (`UserWidget.AddToViewport` (`self.WD_Fade`) 0)
  (`UserWidget.PlayAnimation` (`self.WD_Fade`) (`self.Anime_FadeOut`) 0.0 1 "Forward" 1.0)
  (add `WidgetAnimation.OnAnimationFinished` (`self.Anime_FadeOut`) (delegate `Event_AnimeFIn_FadeOut`)))

(event `Event_AnimeFIn_FadeIn`
  ;[1 1 1] Fade In
  (set `self.IsFadeInFin` true)
  (`Widget.RemoveFromParent` (`self.WD_Fade`)))

(event `Event_AnimeFIn_FadeOut`
  ;[1 1 1] Fade Out
  (set `self.IsFadeOutFin` true))

(event `self.ReceiveTick`
  (params (DeltaSeconds :type "Float (single-precision)"))
  ;[1 1 1] Jump To LoadLevel
  (bind _asmy_game_instance (cast `/Game/Contents/Blueprint/MyGameInstance` (`GameplayStatics.GetGameInstance`)))
  (if (`/Game/Contents/Blueprint/MyGameInstance.JumpLevel` _asmy_game_instance)
    (if (`self.IsFadeOutFin`)
      (`GameplayStatics.OpenLevel` "level_load"))))

(fn `UserConstructionScript`)