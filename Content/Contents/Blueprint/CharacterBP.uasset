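; Flying character Blueprint with dive-and-climb momentum, exposing movement and turning functions that this file does not itself call.
; MoveCharacter speeds up in steep dives and slows otherwise within min/max limits, then feeds speed as scaled input along control rotation and prints velocity.
; MoveRotation applies yaw and pitch input and orients the mesh from velocity through FInterpTo, with the velocity-derived angle passed as Current rather than Target.
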(event `self.ReceiveBeginPlay`
  (set `self.Current Speed` (`self.Min Fly Move Speed`)))

(fn `Move Character`
  (locals (`VectorZ Coefficient` :type "Float (double-precision)"))
  (bind _min_fly_move_speed (`self.Min Fly Move Speed`))
  (bind _max_fly_move_speed (`self.Max Fly Move Speed`))
  (bind _returnvalue (* (`self.Current Speed`) (+ (* (* (`self.Acceleration Fly Move Speed`) 0.4) (* (`local.VectorZ Coefficient`) -0.1)) 1.0)))
  (bind _returnvalue_2 (* (`self.Current Speed`) (- 1.0 (* (* (`self.Deceleration Fly Move Speed`) 0.1) (* (`local.VectorZ Coefficient`) 0.075)))))
  ;[1 1 1] Speed
  (bind _output_get (set `local.VectorZ Coefficient` (.z (`KismetMathLibrary.Normal` (`self.GetVelocity`)))))
  (if (> _output_get -0.5)
    ;[1 1 1] Decelerate
    (if (not (>= (`local.VectorZ Coefficient`) 0.5))
      (set `local.VectorZ Coefficient` 0.3))
    (if (> _returnvalue_2 _min_fly_move_speed)
      (set `self.Current Speed` _returnvalue_2)
      (else
        (set `self.Current Speed` _min_fly_move_speed)))
    ;[1 1 1] Direction
    (`self.AddMovementInput` (`KismetMathLibrary.GetForwardVector` (`KismetMathLibrary.MakeRotator` 0.0 (.pitch (`self.GetControlRotation`)) (.yaw (`self.GetControlRotation`)))) (/ (`self.Current Speed`) (`self.Max Fly Move Speed`)) :!label _label)
    (`KismetSystemLibrary.PrintString` (`KismetStringLibrary.Conv_DoubleToString` (`KismetMathLibrary.VSize` (`self.GetVelocity`))))
    (else
      ;[1 1 1] Accelerate
      (if true
        (if (<= _returnvalue _max_fly_move_speed)
          (set `self.Current Speed` _returnvalue)
          (goto _label)
          (else
            (set `self.Current Speed` _max_fly_move_speed)
            (goto _label)))))))

(fn `Move Rotation`
  (params (`Turn Vector Value` :type "Vector Structure"))
  (bind _returnvalue (`GameplayStatics.GetWorldDeltaSeconds`))
  ;[1 1 1] Yaw(self)
  (`self.AddControllerYawInput` (.z `Turn Vector Value`))
  ;[1 1 1] Pitch(self)
  (`self.AddControllerPitchInput` (.x `Turn Vector Value`))
  (`SceneComponent.K2_SetWorldRotation` (`self.Mesh`) (`KismetMathLibrary.MakeRotator` (`KismetMathLibrary.FInterpTo` (* (.z (`KismetMathLibrary.Normal` (`self.GetVelocity`))) -90.0) (.roll (`SceneComponent.K2_GetComponentRotation` (`self.Mesh`))) _returnvalue 1.0) 0.0 (`KismetMathLibrary.FInterpTo` (+ (.yaw (`KismetMathLibrary.MakeRotFromX` (`KismetMathLibrary.MakeVector` (.x (`KismetMathLibrary.Normal` (`self.GetVelocity`))) (.y (`KismetMathLibrary.Normal` (`self.GetVelocity`)))))) -90.0) (.yaw (`SceneComponent.K2_GetComponentRotation` (`self.Mesh`))) _returnvalue 1.0)) false false))

(fn `UserConstructionScript`
  (set `CharacterMovementComponent.MaxFlySpeed` (`self.Max Fly Move Speed`) (`self.CharacterMovement`))
  (set `CharacterMovementComponent.MaxWalkSpeed` (`self.Max Walk Move Speed`) (`self.CharacterMovement`)))