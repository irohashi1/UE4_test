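; Test player character that flies where it looks, steered by device tilt, with keyboard and mouse movement and look bindings alongside.
; The Tilt event converts gyro Z and X into controller yaw (inverted) and pitch with fixed sensitivity.
; It then sets max fly speed and applies constant forward input along the control pitch and yaw.
; Keyboard movement uses only control yaw, keeping it horizontal.
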(event `InputAxis|MoveFoward`
  (params (AxisValue :type "Float (single-precision)"))
  ;[1 1 1] Movement (Keyboard)
  (`self.AddMovementInput` (`KismetMathLibrary.GetForwardVector` (`KismetMathLibrary.MakeRotator` 0.0 0.0 (.yaw (`self.GetControlRotation`)))) AxisValue))

(event `InputVectorAxis|Tilt`
  (params (AxisValue :type "Vector Structure"))
  ;[1 1 1] Movement
  (`self.Move Rotation` AxisValue)
  (`self.Move Character`))

(event `InputAxis|MoveRight`
  (params (AxisValue :type "Float (single-precision)"))
  ;[1 1 1] Movement (Keyboard)
  (`self.AddMovementInput` (`KismetMathLibrary.GetRightVector` (`KismetMathLibrary.MakeRotator` 0.0 0.0 (.yaw (`self.GetControlRotation`)))) AxisValue))

(event `InputAxis|Turn`
  (params (AxisValue :type "Float (single-precision)"))
  ;[1 1 1] Camera(Keyboard, Mouse)
  (`self.AddControllerYawInput` AxisValue))

(event `InputAxis|LookUp`
  (params (AxisValue :type "Float (single-precision)"))
  ;[1 1 1] Camera(Keyboard, Mouse)
  (`self.AddControllerPitchInput` AxisValue))

(event `InputAxis|TurnRate`
  (params (AxisValue :type "Float (single-precision)"))
  ;[1 1 1] Camera(Keyboard, Mouse)
  (`self.AddControllerYawInput` AxisValue))

(event `InputAxis|LookUpRate`
  (params (AxisValue :type "Float (single-precision)"))
  ;[1 1 1] Camera(Keyboard, Mouse)
  (`self.AddControllerPitchInput` AxisValue))

(fn `Move Character`
  (locals (`Scale Move Speed` :type "Float (double-precision)"))
  ;[1 1 1] Speed
  (set `CharacterMovementComponent.MaxFlySpeed` 500.0 (`self.CharacterMovement`))
  ;[1 1 1] Direction
  (`self.AddMovementInput` (`KismetMathLibrary.GetForwardVector` (`KismetMathLibrary.MakeRotator` 0.0 (.pitch (`self.GetControlRotation`)) (.yaw (`self.GetControlRotation`)))) 1.0))

(fn `Move Rotation`
  (params (`Jyro Value` :type "Vector Structure"))
  ;[1 1 1] Yaw
  (`self.AddControllerYawInput` (* (`KismetMathLibrary.DegreesToRadians` (* (`KismetMathLibrary.RadiansToDegrees` (.z `Jyro Value`)) -1.0)) 3.0))
  ;[1 1 1] Pitch
  (`self.AddControllerPitchInput` (* (`KismetMathLibrary.DegreesToRadians` (+ (`KismetMathLibrary.RadiansToDegrees` (.x `Jyro Value`)) 0.0)) 3.0)))

(fn `UserConstructionScript`)