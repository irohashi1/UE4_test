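; Goal actor that registers characters finishing after they have passed a checkpoint.
; On overlap it casts the other actor to CharacterBP and checks its CheckPointFlag.
; A valid arrival increments GoalCount, sets IsPlayerGoal if the actor is a PlayerBP, and prints a debug success string.
; The flag is only read here, so repeat overlaps by the same character count again while it stays set.
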(event `self.ReceiveActorBeginOverlap`
  (params (OtherActor :type "Actor Object Reference"))
  (set `self.OtherActorRef` OtherActor)
  ;[1 1 1] OverlapしたActorに対する処理
  (bind _ascharacter_bp (cast `/Game/Contents/Blueprint/CharacterBP` (`self.OtherActorRef`)))
  (if (`/Game/Contents/Blueprint/CharacterBP.Check Point Flag` _ascharacter_bp)
    ;[1 1 1] Goal Count
    (`/Engine/EditorBlueprintResources/StandardMacros.IncrementInt` (`self.GoalCount`)
      (:`  `
        (cast `/Game/Contents/Blueprint/PlayerBP` (`self.OtherActorRef`)
          (:`then`
            (set `self.IsPlayerGoal` true))
          (:`CastFailed`
            _))
        (`KismetSystemLibrary.PrintString` "Suc")))))

(fn `UserConstructionScript`)